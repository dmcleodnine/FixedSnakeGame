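; BP_Food is a food actor whose sprite and score value decay over time after it spawns.
; On BeginPlay it calls SetFood with the first food type, which sets the FoodSprite and Score for that stage.
; Each stage waits on a shrinking Delay, then calls SetFood with the next, lower-scoring type until it reaches the final, cheapest one and stays there.
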(event Custom|Set%20Food
  (params (Type :type FoodColor_Enum%20Enum :default "NewEnumerator0"))
  (bind _foodsprite (Variables|Default|GetFoodSprite))
  (switch Utilities|FlowControl|Switch|SwitchonFoodColor_Enum Type
    (:NewEnumerator0
      (Rendering|Components|Sprite|SetSprite _foodsprite "/Game/Sprites/juliopog_Sprite_1.juliopog_Sprite_1")
      (Variables|Default|SetScore 100)
      (Utilities|FlowControl|Delay 3.0)
      (CallFunction|SetFood "NewEnumerator1"))
    (:NewEnumerator1
      (Rendering|Components|Sprite|SetSprite _foodsprite "/Game/Sprites/suh_Sprite_0.suh_Sprite_0")
      (Variables|Default|SetScore 75)
      (Utilities|FlowControl|Delay 2.0)
      (CallFunction|SetFood "NewEnumerator2"))
    (:NewEnumerator2
      (Rendering|Components|Sprite|SetSprite _foodsprite "/Game/Sprites/tuh_Sprite_5.tuh_Sprite_5")
      (Variables|Default|SetScore 50)
      (Utilities|FlowControl|Delay 1.0)
      (CallFunction|SetFood "NewEnumerator3"))
    (:NewEnumerator3
      (Rendering|Components|Sprite|SetSprite _foodsprite "/Game/Sprites/whhat_Sprite_5.whhat_Sprite_5")
      (Variables|Default|SetScore 20))))

(event EventBeginPlay
  (CallFunction|SetFood "NewEnumerator0"))

(fn ConstructionScript)